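; Interactable lantern teleporter that moves the 2D characters to its set spots.
; On interaction it swaps the lantern to its lit sprite, disables the interacting character's input and scales the lantern through a timeline.
; It then fades the camera out, places every 2D_Character_Base at one of three TPSpot locations chosen by character ID, fades back in and restores input.
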(event `self.ReceiveBeginPlay`
  (`parent.ReceiveBeginPlay`)
  (set `self.DefaultScale` (`SceneComponent.K2_GetComponentScale` (`self.Lantern`))))

(event `self.GetInteractedWith`
  (params (CharacterInteracting :type "/Game/Blueprints/Characters/2D_Character_Base Object Reference"))
  (bind _defaultscale (`self.DefaultScale`))
  (bind _playercameramanager (`PlayerController.PlayerCameraManager` (`GameplayStatics.GetPlayerController` 0)))
  (`PaperSpriteComponent.SetSprite` (`self.Lantern`) "/Game/Blueprints/TP/Texture/lanterne_on_Sprite.lanterne_on_Sprite")
  (bind (_direction _newtrack_0) (`Timeline|SwitchToLightLantern`)
    (:`Update`
      (`self.DisableInput` CharacterInteracting (`GameplayStatics.GetPlayerController` 0))
      (`SceneComponent.SetWorldScale3D` (`self.Lantern`) (`KismetMathLibrary.VLerp` _defaultscale (* _defaultscale (`self.ScaleModifierOnLight`)) _newtrack_0)))
    (:`Finished`
      (`PlayerCameraManager.StartCameraFade` :`self` _playercameramanager :`FromAlpha` 0.0 :`ToAlpha` 1.0 :`Duration` 0.5 :`bHoldWhenFinished` true)
      (`KismetSystemLibrary.Delay` 0.7)
      (bind _outactors (`GameplayStatics.GetAllActorsOfClass` "/Game/Blueprints/Characters/2D_Character_Base.2D_Character_Base_C"))
      (for _array_element _outactors
        (bind _id (`/Game/Blueprints/Characters/2D_Character_Base.ID` _array_element))
        (if (== _id 0)
          (`self.K2_SetActorLocation` _array_element (`SceneComponent.K2_GetComponentLocation` (`self.TPSpot1`)) false false)
          (elif (== _id 1)
            (`self.K2_SetActorLocation` _array_element (`SceneComponent.K2_GetComponentLocation` (`self.TPSpot2`)) false false)
            (elif (== _id 2)
              (`self.K2_SetActorLocation` _array_element (`SceneComponent.K2_GetComponentLocation` (`self.TPSpot3`)) false false)))))
      (`PlayerCameraManager.StartCameraFade` :`self` _playercameramanager :`FromAlpha` 1.0 :`ToAlpha` 0.0 :`Duration` 0.5)
      (`self.EnableInput` CharacterInteracting (`GameplayStatics.GetPlayerController` 0)))))

(fn `UserConstructionScript`
  (`parent.UserConstructionScript`))