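; Deadzone is a kill zone that restarts the current level when a 2D_Character_Base overlaps it.
; On the first such overlap it disables input and spawns a hidden, immobile copy of the character at that spot as a blended view target, detaching the view from the original character.
; It plays a water splash, fades the screen out and, after a short delay, reloads the level by name.
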(event `self.ReceiveActorBeginOverlap`
  (params (OtherActor :type "Actor Object Reference"))
  (bind _returnvalue (`GameplayStatics.GetPlayerController` 0))
  (if (not (`self.Killed`))
    (bind _as2d_character_base (cast `/Game/Blueprints/Characters/2D_Character_Base` OtherActor))
    (set `self.Killed` true)
    (bind _returnvalue_2 (`|SpawnActorFromClass` "/Game/Blueprints/Characters/2D_Character_Base.2D_Character_Base_C" (`self.GetTransform` _as2d_character_base) "Undefined" "OverrideRootScale" null null))
    (`SceneComponent.SetVisibility` (`Actor.RootComponent` _returnvalue_2) false true)
    (`CharacterMovementComponent.DisableMovement` (`Character.CharacterMovement` _returnvalue_2))
    (`self.DisableInput` _as2d_character_base _returnvalue)
    (`PlayerController.SetViewTargetWithBlend` _returnvalue _returnvalue_2 0.0 "VTBlend_EaseOut" 2.0 true)
    (`GameplayStatics.PlaySound2D` "/Game/SOund/Effect/Water/WaterSplash.WaterSplash" 1.0 1.0 0.4 null null)
    (`PlayerCameraManager.StartCameraFade` :`self` (`GameplayStatics.GetPlayerCameraManager` 0) :`ToAlpha` 1.0 :`Duration` 0.3 :`bHoldWhenFinished` true)
    (`KismetSystemLibrary.Delay` 1.0)
    (bind _returnvalue_3 (`GameplayStatics.GetCurrentLevelName` true))
    (`GameplayStatics.OpenLevel` (`KismetStringLibrary.Conv_StringToName` _returnvalue_3))))

(fn `UserConstructionScript`)