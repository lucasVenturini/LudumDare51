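; Interactible actor that loops a StaticMesh back and forth between the start and end points of a Spline.
; Interaction toggles between launching and pausing the movement, and EndInteraction toggles it again when CanBeReactivated is false.
; A fixed timeline uses only its last DurationMovement seconds before the 60-second mark, remapped by GetAlpha into an ease-in-out lerp.
; Timeline updates trigger a direction reversal at either bound of that window.
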(event `self.ReceiveBeginPlay`
  (`self.BeginTime`))

(event `self.ReceiveEndInteraction`
  (if (not (`self.CanBeReactivated`))
    (if (`self.IsPaused`) :!label _label
      (set `self.IsPaused` false)
      (`self.LaunchTimeline`)
      (else
        (set `self.IsPaused` true)
        (`self.PauseTheTimeline`)))))

(event `self.ReceiveInteraction`
  (params (CharacterInteracting :type "/Game/Blueprints/Characters/2D_Character_Base Object Reference"))
  (goto _label))

(event `LaunchTimeline`
  (bind _spline (`self.Spline`))
  (if (`self.CurrentTargetIsB`)
    (bind (_direction _newtrack_0) (`Timeline|Timeline_0` :`NewTime` (- 60.0 (`self.DurationMovement`)) :!label _label_2)
      (:`Update`
        (if (`self.FirstLaunch`)
          (set `self.FirstLaunch` false)
          (else
            (set `self.CurrentTime` _newtrack_0)
            (`SceneComponent.K2_SetWorldLocation` (`self.StaticMesh`) (`KismetMathLibrary.VLerp` (`SplineComponent.GetLocationAtDistanceAlongSpline` _spline 0.0 "World") (`SplineComponent.GetLocationAtDistanceAlongSpline` _spline (`SplineComponent.GetSplineLength` _spline) "World") (`|EaseFunction` "EaseInOut" (`self.GetAlpha` _newtrack_0) 0.0 1.0)) false false)
            (if (>= (`self.CurrentTime`) (- 60.0 (`self.DurationMovement`)))
              (if (>= (`self.CurrentTime`) 60.0)
                (`KismetSystemLibrary.PrintString` "REVERSE")
                (`self.Reverse_Timeline`))
              (else
                (`KismetSystemLibrary.PrintString` "REVERSE")
                (`self.Reverse_Timeline`)))))))
    (else
      (goto _label_2 :!via `Reverse`))))

(event `PauseTheTimeline`
  (goto _label_2 :!via `Stop`))

(event `Reverse_Timeline`
  (set `self.CurrentTargetIsB` (not (`self.CurrentTargetIsB`)))
  (if (`self.CurrentTargetIsB`)
    (goto _label_2)
    (else
      (goto _label_2 :!via `Reverse`))))

(event `BeginTime`
  (goto _label_2 :!via `SetNewTime`))

(fn `GetAlpha`
  (params (in :type "Float (double-precision)"))
  (returns (Alpha :type "Float (double-precision)"))
  (return (/ (- in (- 60.0 (`self.DurationMovement`))) (`self.DurationMovement`))))

(fn `UserConstructionScript`
  (`parent.UserConstructionScript`))