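; Interactible button actor that moves its Cube1 mesh down and back up in response to overlaps.
; Begin overlap plays a timeline when IsAnActiveButton is true, while end overlap reverses it only when that flag is false.
; The timeline linearly eases the cube from its BeginPlay world position to a lowered position, with the drop scaled by actor scale.
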(event `self.ReceiveBeginPlay`
  (`parent.ReceiveBeginPlay`)
  (set `self.Initial World Location` (`SceneComponent.K2_GetComponentLocation` (`self.Cube1`))))

(event `self.ReceiveActorBeginOverlap`
  (params (OtherActor :type "Actor Object Reference"))
  (`parent.ReceiveActorBeginOverlap` OtherActor)
  (if (`self.IsAnActiveButton`)
    (set `self.CurrentTargetIsB` true)
    (`self.LaunchTimeline`)))

(event `self.ReceiveActorEndOverlap`
  (params (OtherActor :type "Actor Object Reference"))
  (`parent.ReceiveActorEndOverlap` OtherActor)
  (if (not (`self.IsAnActiveButton`))
    (set `self.CurrentTargetIsB` false)
    (`self.LaunchTimeline`)))

(event `LaunchTimeline`
  (if (`self.CurrentTargetIsB`)
    (bind (_direction _newtrack_0) (`Timeline|Timeline_0` :!label _label)
      (:`Update`
        (`SceneComponent.K2_SetWorldLocation` (`self.Cube1`) (`|EaseFunction` "Linear" _newtrack_0 (`self.Initial World Location`) (- (`self.Initial World Location`) (* (`self.GetActorScale3D`) (0.0 0.0 20.0)))) false false)))
    (else
      (goto _label :!via `Reverse`))))

(fn `UserConstructionScript`
  (`parent.UserConstructionScript`))