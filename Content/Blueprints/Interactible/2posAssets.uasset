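; Interactible actor that moves a static mesh back and forth between the start and end points of a spline.
; Each Interaction toggles the target end and plays or reverses a timeline, whose updates lerp the mesh's world location with ease-in-out.
; DurationMovement sets travel time by using only the final stretch of a fixed 60-second timeline, remapped by GetAlpha and stopped at that window's lower bound.
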(event `self.ReceiveInteraction`
  (params (CharacterInteracting :type "/Game/Blueprints/Characters/2D_Character_Base Object Reference"))
  (if (`self.CurrentTargetIsB`)
    (set `self.CurrentTargetIsB` false)
    (else
      (set `self.CurrentTargetIsB` true)))
  (`self.LaunchTimeline`))

(event `LaunchTimeline`
  (bind _spline (`self.Spline`))
  (if (`self.CurrentTargetIsB`)
    (if (< (`self.CurrentTime`) 60.0)
      (bind (_direction _newtrack_0) (`Timeline|Timeline_0` :`NewTime` (- 60.0 (`self.DurationMovement`)) :!label _label)
        (:`Update`
          (set `self.CurrentTime` _newtrack_0)
          (`SceneComponent.K2_SetWorldLocation` (`self.StaticMesh`) (`KismetMathLibrary.VLerp` (`SplineComponent.GetLocationAtDistanceAlongSpline` _spline 0.0 "World") (`SplineComponent.GetLocationAtDistanceAlongSpline` _spline (`SplineComponent.GetSplineLength` _spline) "World") (`|EaseFunction` "EaseInOut" (`self.GetAlpha` _newtrack_0) 0.0 1.0)) false false)
          (if (not (> (`self.CurrentTime`) (- 60.0 (`self.DurationMovement`))))
            (`self.StopTimeline`)))))
    (elif (> (`self.CurrentTime`) (- 60.0 (`self.DurationMovement`)))
      (goto _label :!via `Reverse`))))

(event `StopTimeline`
  (goto _label :!via `Stop`))

(event `self.ReceiveBeginPlay`
  (goto _label :!via `SetNewTime`))

(fn `GetAlpha`
  (params (in :type "Float (double-precision)"))
  (returns (Alpha :type "Float (double-precision)"))
  (return (/ (- in (- 60.0 (`self.DurationMovement`))) (`self.DurationMovement`))))

(fn `UserConstructionScript`
  (`parent.UserConstructionScript`))