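; Lever is an interactible actor whose sprite swings between two positions each time it is interacted with.
; It extends a parent interactible, passing overlap and interaction events up before acting.
; Each interaction flips the CurrentTargetIsB flag, then plays or reverses a timeline that linearly blends the lever sprite's world rotation between two fixed pitch angles.
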(event `self.ReceiveBeginPlay`
  (`parent.ReceiveBeginPlay`))

(event `self.ReceiveActorBeginOverlap`
  (params (OtherActor :type "Actor Object Reference"))
  (`parent.ReceiveActorBeginOverlap` OtherActor))

(event `self.GetInteractedWith`
  (params (CharacterInteracting :type "/Game/Blueprints/Characters/2D_Character_Base Object Reference"))
  (`parent.GetInteractedWith` null)
  (if (`self.CurrentTargetIsB`)
    (set `self.CurrentTargetIsB` false)
    (else
      (set `self.CurrentTargetIsB` true)))
  (`self.LaunchTimeline`))

(event `self.ReceiveActorEndOverlap`
  (params (OtherActor :type "Actor Object Reference"))
  (`parent.ReceiveActorEndOverlap` OtherActor))

(event `LaunchTimeline`
  (if (`self.CurrentTargetIsB`)
    (bind (_direction _newtrack_0) (`Timeline|Timeline_0` :!label _label)
      (:`Update`
        (`SceneComponent.K2_SetWorldRotation` (`self.levier_Sprite`) (`|EaseFunction` "Linear" _newtrack_0 (struct :`Pitch` -20.0) (struct :`Pitch` 70.0)) false false)))
    (else
      (goto _label :!via `Reverse`))))

(fn `UserConstructionScript`
  (`parent.UserConstructionScript`))