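; Interactor is an overlap trigger that relays interactions from 2D characters to the objects in its Interactible array.
; With ActivateByRange it fires on overlap and stops on exit; otherwise it registers with the character as an available interactor.
; Leaving always removes it from the character.
; Characters whose ID is in ForbiddenCharacter neither start nor end interactions on those objects.
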(event `self.ReceiveActorBeginOverlap`
  (params (OtherActor :type "Actor Object Reference"))
  (bind _as2d_character_base (cast `/Game/Blueprints/Characters/2D_Character_Base` OtherActor))
  (if (`self.ActivateByRange`)
    (`self.GetInteractedWith` _as2d_character_base)
    (else
      (`/Game/Blueprints/Characters/2D_Character_Base.ReceiveNewInteractor` _as2d_character_base self))))

(event `self.ReceiveActorEndOverlap`
  (params (OtherActor :type "Actor Object Reference"))
  (bind _as2d_character_base (cast `/Game/Blueprints/Characters/2D_Character_Base` OtherActor))
  (if (`self.ActivateByRange`)
    (`self.StopInteracting` _as2d_character_base)
    (`/Game/Blueprints/Characters/2D_Character_Base.RemoveInteractor` _as2d_character_base self)
    (else
      (`/Game/Blueprints/Characters/2D_Character_Base.RemoveInteractor` _as2d_character_base self))))

(event `GetInteractedWith`
  (params (CharacterInteracting :type "/Game/Blueprints/Characters/2D_Character_Base Object Reference"))
  (for _array_element (`self.Interactible`)
    (if (not (`KismetArrayLibrary.Array_Contains` (`self.ForbiddenCharacter`) (`/Game/Blueprints/Characters/2D_Character_Base.ID` CharacterInteracting)))
      (`/Game/Blueprints/Interactible/AbstractClass/Interactible.ReceiveInteraction` _array_element CharacterInteracting))))

(event `StopInteracting`
  (params (`Charactere Stopping` :type "/Game/Blueprints/Characters/2D_Character_Base Object Reference"))
  (for _array_element (`self.Interactible`)
    (if (not (`KismetArrayLibrary.Array_Contains` (`self.ForbiddenCharacter`) (`/Game/Blueprints/Characters/2D_Character_Base.ID` `Charactere Stopping`)))
      (`/Game/Blueprints/Interactible/AbstractClass/Interactible.ReceiveEndInteraction` _array_element))))

(fn `UserConstructionScript`)