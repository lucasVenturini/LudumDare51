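; A 2D Paper2D player character that moves along world X and Y from directional axis inputs.
; Each tick it switches the sprite flipbook between run and idle based on velocity magnitude.
; It also sets controller yaw from the X velocity sign to face left or right, defaulting to right when X velocity is zero.
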(event `self.ReceiveTick`
  (params (DeltaSeconds :type "Float (single-precision)"))
  (`self.UpdateAnimation`)
  (`self.UpdateControllerRotation`))

(event `InputAxis|InputRight`
  (params (AxisValue :type "Float (single-precision)"))
  (`self.AddMovementInput` (1.0 0.0 0.0) AxisValue))

(event `InputAxis|InputLeft`
  (params (AxisValue :type "Float (single-precision)"))
  (`self.AddMovementInput` (-1.0 0.0 0.0) AxisValue))

(event `InputAxis|InputUp`
  (params (AxisValue :type "Float (single-precision)"))
  (`self.AddMovementInput` (0.0 -1.0 0.0) AxisValue))

(event `InputAxis|InputDown`
  (params (AxisValue :type "Float (single-precision)"))
  (`self.AddMovementInput` (0.0 1.0 0.0) AxisValue))

(event `UpdateAnimation`
  (`PaperFlipbookComponent.SetFlipbook` (`self.Sprite`) (select `bool` (> (`KismetMathLibrary.VSize` (`MovementComponent.Velocity` (`self.CharacterMovement`))) 0.5) :`false` "/Game/2DAssets/PlaceHolderAssets/FoxIdle/player-idle.player-idle" :`true` "/Game/2DAssets/PlaceHolderAssets/FoxRun/player-run.player-run" :!type "PaperFlipbook Object Reference")))

(event `UpdateControllerRotation`
  (`/Engine/EditorBlueprintResources/StandardMacros.CompareFloat` (.x (`MovementComponent.Velocity` (`self.CharacterMovement`)))
    (:`>`
      (`Controller.SetControlRotation` (`self.GetController`) (`KismetMathLibrary.MakeRotator` 0.0) :!label _label))
    (:`==`
      (goto _label))
    (:`<`
      (`Controller.SetControlRotation` (`self.GetController`) (`KismetMathLibrary.MakeRotator` 0.0 0.0 180.0)))))

(fn `UserConstructionScript`)