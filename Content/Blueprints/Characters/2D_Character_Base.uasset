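; Base 2D flipbook character for a switchable-player game, with four-direction movement and jumping.
; Tick selects idle, run or falling flipbooks, flips control yaw by horizontal velocity and line-traces down to place a floor decal.
; Timelines squash and stretch the sprite on jump and landing.
; The switch input cycles a shared possessed ID through the OtherPlayer array, blends the camera to that character, then possesses it after the blend.
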(event `self.ReceiveBeginPlay`
  (set `self.ScaleInitial` (`SceneComponent.K2_GetComponentScale` (`self.Sprite`))))

(event `self.ReceiveTick`
  (params (DeltaSeconds :type "Float (single-precision)"))
  (`self.UpdateAnimation`)
  (`self.UpdateControllerRotation`)
  (`self.DecaleOnTheFloor`))

(event `InputAxis|InputRight`
  (params (AxisValue :type "Float (single-precision)"))
  (`self.AddMovementInput` (1.0 0.0 0.0) AxisValue))

(event `InputAxis|InputLeft`
  (params (AxisValue :type "Float (single-precision)"))
  (`self.AddMovementInput` (-1.0 0.0 0.0) AxisValue))

(event `InputAxis|InputUp`
  (params (AxisValue :type "Float (single-precision)"))
  (`self.AddMovementInput` (0.0 -1.0 0.0) AxisValue))

(event `InputAxis|InputDown`
  (params (AxisValue :type "Float (single-precision)"))
  (`self.AddMovementInput` (0.0 1.0 0.0) AxisValue))

(event `UpdateAnimation`
  (`PaperFlipbookComponent.SetFlipbook` (`self.Sprite`) (select `bool` (> (`KismetMathLibrary.VSize` (`MovementComponent.Velocity` (`self.CharacterMovement`))) 0.5) :`false` "/Game/2DAssets/PlaceHolderAssets/FoxIdle/player-idle.player-idle" :`true` "/Game/2DAssets/PlaceHolderAssets/FoxRun/player-run.player-run" :!type "PaperFlipbook Object Reference"))
  (if (`NavMovementComponent.IsFalling` (`self.CharacterMovement`))
    (`PaperFlipbookComponent.SetFlipbook` (`self.Sprite`) "/Game/2DAssets/PlaceHolderAssets/FoxFall/FoxFalling.FoxFalling")))

(event `UpdateControllerRotation`
  (`/Engine/EditorBlueprintResources/StandardMacros.CompareFloat` (.x (`MovementComponent.Velocity` (`self.CharacterMovement`)))
    (:`>`
      (`Controller.SetControlRotation` (`self.GetController`) (`KismetMathLibrary.MakeRotator` 0.0)))
    (:`<`
      (`Controller.SetControlRotation` (`self.GetController`) (`KismetMathLibrary.MakeRotator` 0.0 0.0 180.0)))))

(event `InputAction|InputJump`
  (params (Key :type "Key Structure"))
  (:`Pressed`
    (`self.Jump`)
    (`self.StretchJump`))
  (:`Released`
    (`self.StopJumping`)))

(event `self.OnLanded`
  (params (Hit :type "HitResult Structure (by ref)"))
  (`self.SretchLand`))

(event `InputAction|switch`
  (params (Key :type "Key Structure"))
  (bind _output (`|GetArrayItem` (`self.OtherPlayer`) (`self.PossesedID`)))
  (:`Pressed`
    (if (== (`self.ID`) (`self.PossesedID`))
      (if (== (+ (`self.PossesedID`) 1) (`KismetArrayLibrary.Array_Length` (`self.OtherPlayer`)))
        (`self.SetPossedIDForAll` 0)
        (else
          (`self.SetPossedIDForAll` (+ (`self.PossesedID`) 1))))
      (`PlayerController.SetViewTargetWithBlend` (`GameplayStatics.GetPlayerController` 0) (`|GetArrayItem` (`self.OtherPlayer`) (`self.PossesedID`)) (`self.Blend Time`) "VTBlend_EaseOut" 2.0 true)
      (`self.DisableInput` (`GameplayStatics.GetPlayerController` 0))
      (set `MovementComponent.Velocity` (0.0 0.0 0.0) (`self.CharacterMovement`))
      (`KismetSystemLibrary.Delay` (`self.Blend Time`))
      (`GameplayStatics.SetGlobalTimeDilation` 1.0)
      (`Controller.Possess` (`GameplayStatics.GetPlayerController` 0) _output)
      (`self.EnableInput` _output (`GameplayStatics.GetPlayerController` 0)))))

(event `StretchJump`
  (bind (_direction _newtrack_0) (`Timeline|JumpSqueeze` :!via `PlayFromStart`)
    (:`Update`
      (`SceneComponent.SetRelativeScale3D` (`self.Sprite`) (`KismetMathLibrary.VLerp` (`self.ScaleInitial`) (* (`self.ScaleInitial`) (`self.JumpScaleModifier`)) _newtrack_0)))))

(event `SretchLand`
  (bind (_direction _newtrack_0) (`Timeline|Timeline_0` :!via `PlayFromStart`)
    (:`Update`
      (`SceneComponent.SetRelativeScale3D` (`self.Sprite`) (`KismetMathLibrary.VLerp` (`self.ScaleInitial`) (* (`self.ScaleInitial`) (`self.LandScaleModifier`)) _newtrack_0)))))

(event `DecaleOnTheFloor`
  (bind _outhit (`KismetSystemLibrary.LineTraceSingle` (`SceneComponent.K2_GetComponentLocation` (`self.Sprite`)) (- (`SceneComponent.K2_GetComponentLocation` (`self.Sprite`)) (0.0 0.0 1000.0)) "TraceTypeQuery1"))
  (`SceneComponent.K2_SetWorldLocation` (`self.Decal`) (`.Location` (`GameplayStatics.BreakHitResult` _outhit)) false false))

(fn `SetPossedIDForAll`
  (params (NewID :type Integer))
  (for _array_element (`self.OtherPlayer`)
    (set `/Game/Blueprints/Characters/2D_Character_Base.PossesedID` NewID _array_element)))

(fn `UserConstructionScript`)