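; Actor Blueprint that continuously rotates its static mesh back and forth between its starting world rotation and RotationTarget.
; BeginPlay caches the initial rotation, and Tick sets the world rotation with an EaseInOut blend between the two.
; The blend alpha is a triangle wave computed from game time modulo Period, so motion needs no timeline and instances with equal periods stay in phase.
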(event `self.ReceiveBeginPlay`
  (set `self.InitialRotation` (`SceneComponent.K2_GetComponentRotation` (`self.StaticMesh`))))

(event `self.ReceiveTick`
  (params (DeltaSeconds :type "Float (single-precision)"))
  (bind _remainder (`KismetMathLibrary.FMod` (`KismetSystemLibrary.GetGameTimeInSeconds`) (`self.Period`)))
  (bind _returnvalue (/ (`self.Period`) 2.0))
  (`SceneComponent.K2_SetWorldRotation` (`self.StaticMesh`) (`|EaseFunction` "EaseInOut" (`KismetMathLibrary.SelectFloat` (/ _remainder _returnvalue) (- 1.0 (/ (- _remainder _returnvalue) _returnvalue)) (> (/ (`self.Period`) 2.0) _remainder)) (`self.InitialRotation`) (`self.RotationTarget`)) false false))

(fn `UserConstructionScript`)