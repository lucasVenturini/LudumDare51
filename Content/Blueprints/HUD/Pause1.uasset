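; Pause1 is an actor Blueprint that opens the MainMenu widget and pauses the game as soon as it begins play.
; BeginPlay creates the widget, adds it to the viewport, pauses, switches input to game and UI, and shows the mouse cursor.
; An unconnected chain that would remove the menu, restore game-only input, hide the cursor and unpause never runs, so this asset does not close the menu itself.
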(event `self.ReceiveBeginPlay`
  (bind _returnvalue (`GameplayStatics.GetPlayerController` 0))
  (bind _returnvalue_2 (`|CreateWidget` "/Game/Blueprints/HUD/MainMenu.MainMenu_C"))
  (`UserWidget.AddToViewport` _returnvalue_2 0)
  (`GameplayStatics.SetGamePaused` true)
  (`WidgetBlueprintLibrary.SetInputMode_GameAndUIEx` _returnvalue null)
  (set `PlayerController.bShowMouseCursor` true _returnvalue))

(fn `UserConstructionScript`)