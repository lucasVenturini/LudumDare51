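; Pause is an actor Blueprint that toggles the game's pause menu from the Pause input action.
; A FlipFlop alternates each press between creating a new Menu widget with the game paused, and removing that widget with the game resumed.
; Each toggle also switches the first player controller between Game and UI and Game Only input modes, showing or hiding the mouse cursor to match.
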(event `InputAction|Pause` :paused true
  (params (Key :type "Key Structure"))
  (bind _returnvalue (`GameplayStatics.GetPlayerController` 0))
  (bind _returnvalue_2 (`GameplayStatics.GetPlayerController` 0))
  (:`Pressed`
    (`/Engine/EditorBlueprintResources/StandardMacros.FlipFlop`
      (:`A`
        (bind _returnvalue_3 (`|CreateWidget` "/Game/Blueprints/HUD/Menu.Menu_C"))
        (`UserWidget.AddToViewport` _returnvalue_3 0)
        (`GameplayStatics.SetGamePaused` true)
        (`WidgetBlueprintLibrary.SetInputMode_GameAndUIEx` _returnvalue null)
        (set `PlayerController.bShowMouseCursor` true _returnvalue))
      (:`B`
        (`Widget.RemoveFromParent` _returnvalue_3)
        (`WidgetBlueprintLibrary.SetInputMode_GameOnly` _returnvalue_2)
        (set `PlayerController.bShowMouseCursor` false _returnvalue_2)
        (`GameplayStatics.SetGamePaused` false)))))

(fn `UserConstructionScript`)