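; In-game HUD that shows the chrono widget at start and manages tutorial prompts, end-level screens and the pause menu.
; Add and remove events toggle the lever, carry and altar tutorial widgets, using flags to avoid duplicates.
; Four EndLevel events clear all widgets, create the same EndLevel0 widget and animate its image alpha through separate timelines.
; Pause input opens the menu through a FlipFlop with only the pausing branch wired.
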(event `self.ReceiveBeginPlay`
  (bind _returnvalue (`|CreateWidget` "/Game/Blueprints/Chrono/ChronoWidget.ChronoWidget_C"))
  (`UserWidget.AddToViewport` _returnvalue 0))

(event `EndLevel3`
  (`WidgetLayoutLibrary.RemoveAllWidgets`)
  (bind _returnvalue (`|CreateWidget` "/Game/Blueprints/EndLevel/EndLevelWidget/EndLevel0.EndLevel0_C"))
  (`Image.SetBrushTintColor` (`/Game/Blueprints/EndLevel/EndLevelWidget/EndLevel0.Image_20` _returnvalue) (make `SlateColor` (make `LinearColor` 1.0 1.0 1.0)))
  (`UserWidget.AddToViewport` _returnvalue 0)
  (bind (_direction _newtrack_0) (`Timeline|Timeline_2`)
    (:`Update`
      (`Image.SetBrushTintColor` (`/Game/Blueprints/EndLevel/EndLevelWidget/EndLevel0.Image_20` _returnvalue) (make `SlateColor` (make `LinearColor` 1.0 1.0 1.0 _newtrack_0))))))

(event `EndLevel2`
  (`WidgetLayoutLibrary.RemoveAllWidgets`)
  (bind _returnvalue (`|CreateWidget` "/Game/Blueprints/EndLevel/EndLevelWidget/EndLevel0.EndLevel0_C"))
  (`Image.SetBrushTintColor` (`/Game/Blueprints/EndLevel/EndLevelWidget/EndLevel0.Image_20` _returnvalue) (make `SlateColor` (make `LinearColor` 1.0 1.0 1.0)))
  (`UserWidget.AddToViewport` _returnvalue 0)
  (bind (_direction _newtrack_0) (`Timeline|Timeline_1`)
    (:`Update`
      (`Image.SetBrushTintColor` (`/Game/Blueprints/EndLevel/EndLevelWidget/EndLevel0.Image_20` _returnvalue) (make `SlateColor` (make `LinearColor` 1.0 1.0 1.0 _newtrack_0))))))

(event `EndLevel1`
  (`WidgetLayoutLibrary.RemoveAllWidgets`)
  (bind _returnvalue (`|CreateWidget` "/Game/Blueprints/EndLevel/EndLevelWidget/EndLevel0.EndLevel0_C"))
  (`Image.SetBrushTintColor` (`/Game/Blueprints/EndLevel/EndLevelWidget/EndLevel0.Image_20` _returnvalue) (make `SlateColor` (make `LinearColor` 1.0 1.0 1.0)))
  (`UserWidget.AddToViewport` _returnvalue 0)
  (bind (_direction _newtrack_0) (`Timeline|Timeline_0`)
    (:`Update`
      (`Image.SetBrushTintColor` (`/Game/Blueprints/EndLevel/EndLevelWidget/EndLevel0.Image_20` _returnvalue) (make `SlateColor` (make `LinearColor` 1.0 1.0 1.0 _newtrack_0))))))

(event `EndLevel0`
  (`WidgetLayoutLibrary.RemoveAllWidgets`)
  (bind _returnvalue (`|CreateWidget` "/Game/Blueprints/EndLevel/EndLevelWidget/EndLevel0.EndLevel0_C"))
  (`Image.SetBrushTintColor` (`/Game/Blueprints/EndLevel/EndLevelWidget/EndLevel0.Image_20` _returnvalue) (make `SlateColor` (make `LinearColor` 1.0 1.0 1.0)))
  (`UserWidget.AddToViewport` _returnvalue 0)
  (bind (_direction _newtrack_0) (`Timeline|FadeIn`)
    (:`Update`
      (`Image.SetBrushTintColor` (`/Game/Blueprints/EndLevel/EndLevelWidget/EndLevel0.Image_20` _returnvalue) (make `SlateColor` (make `LinearColor` 1.0 1.0 1.0 _newtrack_0))))))

(event `AddHUDLever`
  (if (not (`self.LeverOnViewport`))
    (bind _returnvalue (`|CreateWidget` "/Game/Blueprints/Tutorial/TutoLever.TutoLever_C"))
    (set `self.HUDLever` _returnvalue)
    (`UserWidget.AddToViewport` _returnvalue 0)
    (set `self.LeverOnViewport` true)))

(event `RemoveHUDLever`
  (if (`self.LeverOnViewport`)
    (`Widget.RemoveFromParent` (`self.HUDLever`))
    (set `self.LeverOnViewport` false)))

(event `AddHUDCarry`
  (if (not (`self.CarryOnViewport`))
    (bind _returnvalue (`|CreateWidget` "/Game/Blueprints/Tutorial/TutoCarry.TutoCarry_C"))
    (set `self.CarryHUD` _returnvalue)
    (`UserWidget.AddToViewport` _returnvalue 0)
    (set `self.CarryOnViewport` true)))

(event `EndHUDCarry`
  (if (`self.CarryOnViewport`)
    (`Widget.RemoveFromParent` (`self.CarryHUD`))
    (set `self.CarryOnViewport` false)))

(event `AddHUDAltar`
  (if (not (`self.AltarOnViewport`))
    (bind _returnvalue (`|CreateWidget` "/Game/Blueprints/Tutorial/TutorialAltar.TutorialAltar_C"))
    (set `self.AltarHUD` _returnvalue)
    (`UserWidget.AddToViewport` _returnvalue 0)
    (set `self.AltarOnViewport` true)))

(event `RemoveHUDAltar`
  (if (`self.AltarOnViewport`)
    (`Widget.RemoveFromParent` (`self.AltarHUD`))
    (set `self.AltarOnViewport` false)))

(event `InputAction|Pause` :paused true
  (params (Key :type "Key Structure"))
  (bind _returnvalue (`GameplayStatics.GetPlayerController` 0))
  (:`Pressed`
    (`/Engine/EditorBlueprintResources/StandardMacros.FlipFlop`
      (:`A`
        (bind _returnvalue_2 (`|CreateWidget` "/Game/Blueprints/HUD/Menu.Menu_C"))
        (`UserWidget.AddToViewport` _returnvalue_2 0)
        (`GameplayStatics.SetGamePaused` true)
        (`WidgetBlueprintLibrary.SetInputMode_GameAndUIEx` _returnvalue null)
        (set `PlayerController.bShowMouseCursor` true _returnvalue)))))

(fn `UserConstructionScript`)