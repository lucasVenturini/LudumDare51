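; EndLevel3 is a trigger actor that ends the third level when the 2D player character overlaps it.
; On overlap it turns off the character's timer switch and fades the camera and audio to black.
; It then calls EndLevel3 on the HUDGame actor, waits, and opens the level named by its Level variable.
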(event `self.ReceiveActorBeginOverlap`
  (params (OtherActor :type "Actor Object Reference"))
  (bind _as2d_character_base (cast `/Game/Blueprints/Characters/2D_Character_Base` OtherActor))
  (set `/Game/Blueprints/Characters/2D_Character_Base.EnableTimerSwitch` false _as2d_character_base)
  (`PlayerCameraManager.StartCameraFade` :`self` (`PlayerController.PlayerCameraManager` (`GameplayStatics.GetPlayerController` 0)) :`ToAlpha` 1.0 :`Duration` 1.0 :`bShouldFadeAudio` true :`bHoldWhenFinished` true)
  (`KismetSystemLibrary.Delay` 1.0)
  (bind _outactors (`GameplayStatics.GetAllActorsOfClass` "/Game/Blueprints/HUD/HUDGame.HUDGame_C"))
  (`/Game/Blueprints/HUD/HUDGame.EndLevel3` (`|GetArrayItem` _outactors))
  (`KismetSystemLibrary.Delay` 5.0)
  (`GameplayStatics.OpenLevel` (`self.Level `)))

(fn `UserConstructionScript`)